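; BP_Player is the flipbook-animated player character, handling movement, jumping, health and dialogue interaction.
; BeginPlay registers the Enhanced Input context and creates the health widget, which damage updates before flagging death at zero health; PlayerDied only prints and is never called here.
; E sends TalkMessage to overlapping BP_Fluvis actors through BPI_Dialogue.
; P flip-flops between pause menu and HUD pause-screen widgets, though its only SetGamePaused call passes false.
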(event Input|EnhancedActionEvents|EnhancedInputActionIA_Movement
  (params (ActionValue :type Float%20%28double-precision%29) (ElapsedSeconds :type Float%20%28double-precision%29) (TriggeredSeconds :type Float%20%28double-precision%29) (InputAction :type Input%20Action%20Object%20Reference :default "/Game/Blueprints/IA_Movement.IA_Movement"))
  ;[1 1 1] Enhanced Player Input - movement
  (:Triggered
    (Pawn|Input|AddMovementInput (Transformation|GetActorForwardVector) ActionValue false)
    (Sprite|SetFlipbook (Variables|Default|GetSprite) "/Game/Assets/Anim/FB_Hyrtan_fire_roll.FB_Hyrtan_fire_roll")
    (if (> ActionValue 0.0)
      (Transformation|SetWorldRotation (Variables|Default|GetSprite) "0, 0, 0" false false)
      (else
        (Sprite|SetFlipbook (Variables|Default|GetSprite) "/Game/Assets/Textures/character/Hrytan/FB_Hyrtan_fire_travel_left.FB_Hyrtan_fire_travel_left"))))
  (:Completed
    (Sprite|SetFlipbook (Variables|Default|GetSprite) "/Game/Assets/Anim/FB_Hyrtan_Idle.FB_Hyrtan_Idle")))

(event Input|EnhancedActionEvents|EnhancedInputActionIA_Jump
  (params (ActionValue :type Boolean) (ElapsedSeconds :type Float%20%28double-precision%29) (TriggeredSeconds :type Float%20%28double-precision%29) (InputAction :type Input%20Action%20Object%20Reference :default "/Game/Blueprints/IA_Jump.IA_Jump"))
  ;[1 1 1] Jumping
  (:Triggered
    (Character|Jump))
  (:Completed
    (Character|StopJumping)))

(event EventBeginPlay
  ;[1 1 1] BeginPlay - allow player movment with BP_PlayerController
  (Utilities|FlowControl|Sequence
    (:then_0
      (bind _asbp_player_controller (Utilities|Casting|CastToBP_PlayerController (Pawn|GetController)))
      (Input|AddMappingContext (PlayerController|LocalPlayerSubsystems|GetEnhancedInputLocalPlayerSubsystem _asbp_player_controller) "/Game/Blueprints/IMC_Default.IMC_Default" 0 "(bIgnoreAllPressedKeysUntilRelease=True,bForceImmediately=False)"))
    (:then_1
      ;[1 1 1] print string for debugging
      (Development|PrintString (Utilities|String|ToString(Float) (Variables|Default|GetHealth))))
    (:then_2
      ;[1 1 1] Health System
      ;;[1 1 1] To display health widget on screen
      (bind _returnvalue (UserInterface|CreateWidget "/Game/Assets/Widgets/WBP_PlayerHealthRedo.WBP_PlayerHealthRedo_C"))
      (bind _output_get (Variables|Default|SetHealth%20Widget%20Ref _returnvalue))
      (UserInterface|Viewport|AddtoViewport _output_get 0)
      (CallFunction|UpdateHealth))))

(event Game|Damage|EventAnyDamage
  (params (Damage :type Float%20%28single-precision%29) (DamageType :type Damage%20Type%20Object%20Reference) (InstigatedBy :type Controller%20Object%20Reference) (DamageCauser :type Actor%20Object%20Reference))
  ;[1 1 1] Health System
  (Variables|Default|SetHealth (- (Variables|Default|GetHealth) Damage))
  (CallFunction|UpdateHealth)
  (if (and (<= (Variables|Default|GetHealth) 0.0) (not (Variables|Default|GetIsDead)))
    (Variables|Default|SetIsDead true)))

(event Input|KeyboardEvents|E
  (params (Key :type Key%20Structure :default "None"))
  ;[1 1 1] E keybinding - interact / talk
  (:Pressed
    (for _array_element (Collision|GetOverlappingActors "/Game/Blueprints/BP_Fluvis.BP_Fluvis_C" :!class /Script/Engine.Actor)
      (if (Utilities|DoesObjectImplementInterface _array_element "/Game/Blueprints/BPI_Dialogue.BPI_Dialogue_C")
        (Class|BPIDialogue|Talk(Message) _array_element)))))

(event Input|KeyboardEvents|P
  (params (Key :type Key%20Structure :default "None"))
  (bind _returnvalue (Game|GetPlayerController 0))
  (bind _hud_pause_screen (Variables|Default|GetHUD%20Pause%20Screen))
  ;[1 1 1] PAUSE - keybinding and screen display
  (:Pressed
    (Utilities|FlowControl|FlipFlop
      (:A
        (Widget|RemovefromParent _hud_pause_screen)
        (Game|SetGamePaused false)
        (bind _returnvalue_2 (UserInterface|CreateWidget "/Game/Assets/Widgets/UI/WBP_PauseMenu.WBP_PauseMenu_C"))
        (UserInterface|Viewport|AddtoViewport _returnvalue_2 0))
      (:B
        (UserInterface|Viewport|AddtoViewport _hud_pause_screen 0)
        (Variables|/Script/Engine.PlayerController|SetbShowMouseCursor (Game|GetPlayerController 0) false)
        (Widget|RemovefromParent _returnvalue_2)))
    (Input|SetInputModeGameandUI _returnvalue 0 "DoNotLock" true false)
    (Variables|/Script/Engine.PlayerController|SetbShowMouseCursor _returnvalue false)))

(fn ConstructionScript
  ;[1 1 1] Resets health to default health at start of game
  (Variables|Default|SetHealth (Variables|Default|GetDefaultHealth)))

(fn PlayerDied
  (Development|PrintString "YOu died"))

(fn UpdateHealth
  (Default|UpdateHealth (Variables|Default|GetHealth%20Widget%20Ref) 0.0 (Variables|Default|GetHealth) (Variables|Default|GetDefaultHealth)))