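; Template parent Blueprint for enemies that provides a basic health and death system.
; AnyDamage subtracts damage from Health and, the first time it reaches zero or below, sets IsDead and calls EnemyDead.
; EnemyDead and the construction script are empty stubs.
; Health is not clamped, as the ClampFloat node is left unused.
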(event Game|Damage|EventAnyDamage
  (params (Damage :type Float%20%28single-precision%29) (DamageType :type Damage%20Type%20Object%20Reference) (InstigatedBy :type Controller%20Object%20Reference) (DamageCauser :type Actor%20Object%20Reference))
  ;[1 1 1] Enemy Health System (template)
  (Variables|Default|SetHealth (- (Variables|Default|GetHealth) Damage))
  (if (and (<= (Variables|Default|GetHealth) 0.0) (not (Variables|Default|GetIsDead)))
    (Variables|Default|SetIsDead true)
    (CallFunction|EnemyDead)))

(fn ConstructionScript)

(fn EnemyDead)